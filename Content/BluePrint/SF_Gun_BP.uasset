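; SF_Gun_BP is a gun actor that the player picks up by walking into its box trigger.
; On overlap by player pawn 0 while CanPick is set, it assigns itself as the Ue4ASP_Character's MyGun and calls PickUpGun on that character.
; When the player leaves the box, CanPick is set true after a short delay.
; The construction script starts it pickable and non-laser; this graph never clears CanPick.
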(event `self.Box.OnComponentEndOverlap`
  (params (OverlappedComponent :type "PrimitiveComponent Object Reference") (OtherActor :type "Actor Object Reference") (OtherComp :type "PrimitiveComponent Object Reference") (OtherBodyIndex :type Integer))
  (if (== OtherActor (`GameplayStatics.GetPlayerPawn` 0))
    (`KismetSystemLibrary.Delay` 0.5)
    (set `self.CanPick` true)))

(event `self.Box.OnComponentBeginOverlap`
  (params (OverlappedComponent :type "PrimitiveComponent Object Reference") (OtherActor :type "Actor Object Reference") (OtherComp :type "PrimitiveComponent Object Reference") (OtherBodyIndex :type Integer) (bFromSweep :type Boolean) (SweepResult :type "HitResult Structure (by ref)"))
  (bind _returnvalue (`GameplayStatics.GetPlayerPawn` 0))
  (if (== OtherActor _returnvalue)
    (if (`self.CanPick`)
      (bind _asue_4asp_character (cast `/Game/AnimStarterPack/Ue4ASP_Character` _returnvalue))
      (set `/Game/AnimStarterPack/Ue4ASP_Character.MyGun` self _asue_4asp_character)
      (`/Game/AnimStarterPack/Ue4ASP_Character.PickUpGun` _asue_4asp_character))))

(fn `UserConstructionScript`
  (`parent.UserConstructionScript`)
  (set `self.CanPick` true)
  (set `self.IsLaser` false))