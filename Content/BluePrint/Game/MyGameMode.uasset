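; Multiplayer game mode that sets up joining players and handles respawning.
; On login, the server sorts PlayerStarts into Player1 and Player2 arrays by tag, numbers the player by PlayerArray length, and calls ClientPostLogin on their controller.
; RespawnPlayerEvent destroys the current pawn, then spawns and possesses a new Ue4ASP_Character at a hardcoded transform, ignoring the sorted start points.
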(event `RespawnPlayerEvent`
  (params (PlayerController :type "PlayerController Object Reference"))
  (bind _returnvalue (`Controller.K2_GetPawn` PlayerController))
  (`/Engine/EditorBlueprintResources/StandardMacros.IsValid` _returnvalue
    (:`Is Valid`
      (`self.K2_DestroyActor` _returnvalue))
    (:`Is Not Valid`
      _))
  (bind _returnvalue_2 (`|SpawnActorFromClass` "/Game/AnimStarterPack/Ue4ASP_Character.Ue4ASP_Character_C" (`KismetMathLibrary.MakeTransform` (-690.0 270.0 222.0)) "AdjustIfPossibleButDontSpawnIfColliding" "OverrideRootScale" null null))
  (`Controller.Possess` PlayerController _returnvalue_2))

(event `self.K2_PostLogin`
  (params (NewPlayer :type "PlayerController Object Reference"))
  (`/Engine/EditorBlueprintResources/ActorMacros.Switch Has Authority`
    (:`Authority`
      (bind _outactors (`GameplayStatics.GetAllActorsOfClass` "/Script/Engine.PlayerStart"))
      (for _array_element _outactors
        (if (== (`PlayerStart.PlayerStartTag` _array_element) "Player1")
          (`KismetArrayLibrary.Array_AddUnique` (`self.Player1`) _array_element)
          (else
            (`KismetArrayLibrary.Array_AddUnique` (`self.Player2`) _array_element))))
      (bind _asmy_player_state (cast `/Game/BluePrint/Game/MyPlayerState` (`Controller.PlayerState` NewPlayer)))
      (set `/Game/BluePrint/Game/MyPlayerState.Player Number` (`KismetArrayLibrary.Array_Length` (`GameState.PlayerArray` (`GameplayStatics.GetGameState`))) _asmy_player_state)
      (bind _asmy_player_controller (cast `/Game/BluePrint/Game/MyPlayerController` NewPlayer))
      (`/Game/BluePrint/Game/MyPlayerController.ClientPostLogin` _asmy_player_controller))))

(fn `UserConstructionScript`)