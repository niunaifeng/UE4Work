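; Target1 is a target Blueprint that awards points to the player when its Hit event fires.
; Hit casts player character 0 to Ue4ASP_Character and passes the Increament value to its AddScore function.
; The construction script sets that score value after calling the parent's, and the BeginPlay, overlap and Tick events are disabled stubs.
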(event `self.ReceiveHit`
  (params (MyComp :type "PrimitiveComponent Object Reference") (Other :type "Actor Object Reference") (OtherComp :type "PrimitiveComponent Object Reference") (bSelfMoved :type Boolean) (HitLocation :type "Vector Structure") (HitNormal :type "Vector Structure") (NormalImpulse :type "Vector Structure") (Hit :type "HitResult Structure (by ref)"))
  (bind _asue_4asp_character (cast `/Game/AnimStarterPack/Ue4ASP_Character` (`GameplayStatics.GetPlayerCharacter` 0)))
  (`/Game/AnimStarterPack/Ue4ASP_Character.Add Score` _asue_4asp_character (`self.Increament`)))

(fn `UserConstructionScript`
  (`parent.UserConstructionScript`)
  (set `self.Increament` 10))