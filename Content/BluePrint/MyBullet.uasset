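; MyBullet is an explosive projectile actor that damages player and enemy characters and removes itself five seconds after spawning.
; On hit it damages the character; enemies are also flagged to escape and earn the Shooter 50 points.
; Non-player hits enable gravity and derive friction and bounciness from the inverted physical-material friction.
; Explose hides the sphere, spawns particles and sound, and enlarges the actor before its brief delayed destruction.
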(event `self.ReceiveBeginPlay`
  (`KismetSystemLibrary.Delay` 5.0)
  (`SceneComponent.SetVisibility` (`self.Sphere`) false false)
  (`self.SetActorScale3D` (2.0 2.0 2.0))
  (`KismetSystemLibrary.Delay` 0.01)
  (`self.K2_DestroyActor`))

(event `self.ReceiveTick`
  (params (DeltaSeconds :type "Float (single-precision)")))

(event `self.ReceiveHit`
  (params (MyComp :type "PrimitiveComponent Object Reference") (Other :type "Actor Object Reference") (OtherComp :type "PrimitiveComponent Object Reference") (bSelfMoved :type Boolean) (HitLocation :type "Vector Structure") (HitNormal :type "Vector Structure") (NormalImpulse :type "Vector Structure") (Hit :type "HitResult Structure (by ref)"))
  (bind (_bblockinghit _binitialoverlap _time _distance _location _impactpoint _normal _impactnormal _physmat) (`GameplayStatics.BreakHitResult` Hit))
  (bind _projectilemovement (`self.ProjectileMovement`))
  (bind _returnvalue (- 1.0 (`PhysicalMaterial.Friction` _physmat)))
  (`|ExecutionSequence`
    (:`then_0`
      (bind _asue_4asp_character (cast `/Game/AnimStarterPack/Ue4ASP_Character` Other)
        (:`then`
          (`/Game/AnimStarterPack/Ue4ASP_Character.GetDamage` _asue_4asp_character (`self.Damage`))
          (`self.Explose` :!label _label)
          (`KismetSystemLibrary.Delay` 0.01)
          (`self.K2_DestroyActor`))
        (:`CastFailed`
          (set `ProjectileMovementComponent.ProjectileGravityScale` 1.0 _projectilemovement)
          (if (!= _physmat null)
            (set `ProjectileMovementComponent.Friction` _returnvalue _projectilemovement)
            (set `ProjectileMovementComponent.Bounciness` _returnvalue _projectilemovement))
          (`KismetSystemLibrary.Delay` 0.01)
          (`self.Explose`)
          (`KismetSystemLibrary.Delay` 0.01)
          (`self.K2_DestroyActor`))))
    (:`then_1`
      (bind _asenemy_character (cast `/Game/AI/Enemy_Character` Other))
      (set `/Game/AI/Enemy_Character.ShouldEscape` true _asenemy_character)
      (`/Game/AI/Enemy_Character.GetDamage` _asenemy_character (`self.Damage`))
      (`/Game/AnimStarterPack/Ue4ASP_Character.Add Score` (`self.Shooter`) 50)
      (goto _label))))

(event `PlaySoundExplosion`
  (`GameplayStatics.PlaySoundAtLocation` "/Game/MobileStarterContent/Audio/Explosion01.Explosion01" (`self.K2_GetActorLocation`) (struct) 0.5 1.0 0.0 null null null))

(fn `Explose`
  (`SceneComponent.SetVisibility` (`self.Sphere`) false false)
  (`GameplayStatics.SpawnEmitterAtLocation` "/Game/MobileStarterContent/Particles/P_Explosion.P_Explosion" (`self.K2_GetActorLocation`))
  (`self.PlaySoundExplosion`)
  (`self.SetActorScale3D` (2.0 2.0 2.0)))

(fn `UserConstructionScript`)